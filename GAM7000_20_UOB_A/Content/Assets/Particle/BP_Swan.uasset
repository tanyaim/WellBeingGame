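; BP_Swan is a swan actor that travels along the spline of a referenced swan path.
; On BeginPlay, if ActiveSwan is set, it plays the SwanMover timeline with a rate derived from Duration, starting at SwanStartOffset.
; Each update maps the timeline alpha to a distance along the spline and applies that world-space location and rotation to the actor.
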(event Custom|MoveSwan
  (Components|Timeline|SetPlayRate (Variables|Default|GetSwanMover) (/ 1.0 (Variables|Default|GetDuration)))
  (Components|Timeline|SetNewTime (Variables|Default|GetSwanMover) (Variables|Default|GetSwanStartOffset))
  (bind _alpha (Timeline|SwanMover Play)
    (:Update
      (Variables|Default|SetAlpha _alpha)
      (Transformation|SetActorLocationAndRotation (Spline|GetLocationatDistanceAlongSpline (Variables|/Game/Assets/Particle/BP_SwanPath.BP_SwanPath_C|GetSwanSpline (Variables|Default|GetSwanPathReference)) (Math|Float|Lerp 0.0 (Spline|GetSplineLength (Variables|/Game/Assets/Particle/BP_SwanPath.BP_SwanPath_C|GetSwanSpline (Variables|Default|GetSwanPathReference))) (Variables|Default|GetAlpha)) "World") (Spline|GetRotationatDistanceAlongSpline (Variables|/Game/Assets/Particle/BP_SwanPath.BP_SwanPath_C|GetSwanSpline (Variables|Default|GetSwanPathReference)) (Math|Float|Lerp 0.0 (Spline|GetSplineLength (Variables|/Game/Assets/Particle/BP_SwanPath.BP_SwanPath_C|GetSwanSpline (Variables|Default|GetSwanPathReference))) (Variables|Default|GetAlpha)) "World")))))

(event EventBeginPlay
  (if (Variables|Default|GetActiveSwan)
    (CallFunction|MoveSwan)))

(fn ConstructionScript)