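; Test NPC that accepts a held berry or poppy as a gift from Player1 when F is pressed.
; A Box overlap enables and disables the NPC's input, limiting the key to its vicinity.
; F checks the player's Holding flags, then raises Happiness and Mayor social (though the debug print names the Detective) and hides all four item components.
; The Holding flags are not cleared here.
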(event OnComponentBeginOverlap(Box)
  (params (OverlappedComponent :type Primitive%20Component%20Object%20Reference) (OtherActor :type Actor%20Object%20Reference) (OtherComp :type Primitive%20Component%20Object%20Reference) (OtherBodyIndex :type Integer) (bFromSweep :type Boolean) (SweepResult :type Hit%20Result%20Structure%20%28by%20ref%29))
  ;[1 1 1] Enable/Disable Player Input
  (Input|EnableInput (.ReturnValue (Class|VictoryBPFunctionLibrary|AccessorGetPlayerController (Game|GetPlayerCharacter 0)))))

(event OnComponentEndOverlap(Box)
  (params (OverlappedComponent :type Primitive%20Component%20Object%20Reference) (OtherActor :type Actor%20Object%20Reference) (OtherComp :type Primitive%20Component%20Object%20Reference) (OtherBodyIndex :type Integer))
  ;[1 1 1] Enable/Disable Player Input
  (Input|DisableInput (.ReturnValue (Class|VictoryBPFunctionLibrary|AccessorGetPlayerController (Game|GetPlayerCharacter 0)))))

(event EventBeginPlay
  (bind _asplayer_1 (Utilities|Casting|CastToPlayer1 (Game|GetPlayerCharacter 0)))
  (Variables|Default|SetPlayerRef _asplayer_1))

(event Input|KeyboardEvents|F
  (params (Key :type Key%20Structure))
  (bind _playerref (Variables|Default|GetPlayerRef))
  ;[1 1 1] Give Held Berry
  (:Pressed
    (if (Variables|/Game/Blueprints/Player1.Player1_C|GetHoldingBlackBerry? _playerref)
      (Development|PrintString "Given Detective a gift" :!label _label)
      ;[1 1 1] Adding To Happiness/Social Stat
      (bind _asplayer_1 (Utilities|Casting|CastToPlayer1 (Game|GetPlayerCharacter 0))
        (:then
          (Default|Plus1toHappiness _asplayer_1)
          (Default|Plus1toMayorSocial _asplayer_1)
          (Rendering|SetVisibility (Variables|/Game/Blueprints/Player1.Player1_C|GetBlackberry _asplayer_1) false false))
        (:CastFailed
          (Development|PrintString "Not Working")))
      (elif (Variables|/Game/Blueprints/Player1.Player1_C|GetHoldingBlueBerry? _playerref)
        (goto _label)
        (elif (Variables|/Game/Blueprints/Player1.Player1_C|GetHoldingRaspBerry? _playerref)
          (goto _label)
          (else
            ;[1 1 1] Give Held Flower
            (if (Variables|/Game/Blueprints/Player1.Player1_C|GetHoldingPoppy? (Variables|Default|GetPlayerRef))
              (goto _label))))))))

(fn ConstructionScript)