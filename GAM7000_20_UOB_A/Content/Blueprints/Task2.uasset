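; Task2 is an interactable task actor that the player completes by pressing F while its input is enabled.
; Box overlap begin and end enable and disable the actor's input for player 0's controller, without checking which actor overlaps.
; F sets TaskCompleted, prints a message, casts to Player1 to call Plus1ToEnergy (though commented as happiness), then destroys the Sphere and Box components.
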(event OnComponentBeginOverlap(Box)
  (params (OverlappedComponent :type Primitive%20Component%20Object%20Reference) (OtherActor :type Actor%20Object%20Reference) (OtherComp :type Primitive%20Component%20Object%20Reference) (OtherBodyIndex :type Integer) (bFromSweep :type Boolean) (SweepResult :type Hit%20Result%20Structure%20%28by%20ref%29))
  ;[1 1 1] Enable/Disable Player Input
  (Input|EnableInput (.ReturnValue (Class|VictoryBPFunctionLibrary|AccessorGetPlayerController (Game|GetPlayerCharacter 0)))))

(event OnComponentEndOverlap(Box)
  (params (OverlappedComponent :type Primitive%20Component%20Object%20Reference) (OtherActor :type Actor%20Object%20Reference) (OtherComp :type Primitive%20Component%20Object%20Reference) (OtherBodyIndex :type Integer))
  ;[1 1 1] Enable/Disable Player Input
  (Input|DisableInput (.ReturnValue (Class|VictoryBPFunctionLibrary|AccessorGetPlayerController (Game|GetPlayerCharacter 0)))))

(event Input|KeyboardEvents|F
  (params (Key :type Key%20Structure))
  ;[1 1 1] Completing Task
  (:Pressed
    (Variables|Default|SetTaskCompleted? true)
    (Development|PrintString "Task Completed")
    ;[1 1 1] Adding To Happiness
    (bind _asplayer_1 (Utilities|Casting|CastToPlayer1 (Game|GetPlayerCharacter 0))
      (:then
        (Default|Plus1toEnergy _asplayer_1)
        (Components|DestroyComponent (Variables|Default|GetSphere)))
      (:CastFailed
        (Development|PrintString "Not Working")))))

(fn ConstructionScript)