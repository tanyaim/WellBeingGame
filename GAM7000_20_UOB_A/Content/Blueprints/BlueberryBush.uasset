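; Harvestable blueberry bush that the player picks with the F key to complete a task and gain happiness.
; A box overlap enables or disables the bush's input, so the key only responds nearby.
; Harvesting clears the berry flag, destroys the berry spheres and calls the happiness increment on Player1.
; The first blueberry harvest also hides the journal's UBlueberry element and records the collection on the player.
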(event OnComponentBeginOverlap(Box)
  (params (OverlappedComponent :type Primitive%20Component%20Object%20Reference) (OtherActor :type Actor%20Object%20Reference) (OtherComp :type Primitive%20Component%20Object%20Reference) (OtherBodyIndex :type Integer) (bFromSweep :type Boolean) (SweepResult :type Hit%20Result%20Structure%20%28by%20ref%29))
  ;[1 1 1] Enable/Disable Player Input
  (Input|EnableInput (.ReturnValue (Class|VictoryBPFunctionLibrary|AccessorGetPlayerController (Game|GetPlayerCharacter 0)))))

(event OnComponentEndOverlap(Box)
  (params (OverlappedComponent :type Primitive%20Component%20Object%20Reference) (OtherActor :type Actor%20Object%20Reference) (OtherComp :type Primitive%20Component%20Object%20Reference) (OtherBodyIndex :type Integer))
  ;[1 1 1] Enable/Disable Player Input
  (Input|DisableInput (.ReturnValue (Class|VictoryBPFunctionLibrary|AccessorGetPlayerController (Game|GetPlayerCharacter 0)))))

(event EventBeginPlay
  (bind _asplayer_1 (Utilities|Casting|CastToPlayer1 (Game|GetPlayerCharacter 0)))
  (Variables|Default|SetPlayerReference _asplayer_1))

(event Input|KeyboardEvents|F
  (params (Key :type Key%20Structure :default "None"))
  (bind _playerreference (Variables|Default|GetPlayerReference))
  ;[1 1 1] Completing Task
  (:Pressed
    (if (Variables|Default|GetHasBerries?)
      (Variables|Default|SetHasBerries? false)
      (Variables|Default|SetTaskCompleted? true)
      (Development|PrintString "Task Completed")
      ;[1 1 1] Adding To Happiness
      (bind _asplayer_1 (Utilities|Casting|CastToPlayer1 (Game|GetPlayerCharacter 0))
        (:then
          (Default|Plus1toHappiness _asplayer_1)
          (if (Variables|/Game/Blueprints/Player1.Player1_C|GethasCollectedBlueberry _playerreference)
            _
            (else
              (Class|Image|SetOpacity (Variables|/Game/Journal/Journal.Journal_C|Getu_blueberry (Variables|/Game/Blueprints/Player1.Player1_C|GetJournalReference _playerreference)) 0.0)
              (Variables|/Game/Blueprints/Player1.Player1_C|SethasCollectedBlueberry _playerreference true)))
          (Components|DestroyComponent (Variables|Default|GetSphere))
          (Variables|Default|SetcollectedBerries true))
        (:CastFailed
          (Development|PrintString "Not Working")))
      (else
        (Development|PrintString "Not in harvest")))))

(fn ConstructionScript)