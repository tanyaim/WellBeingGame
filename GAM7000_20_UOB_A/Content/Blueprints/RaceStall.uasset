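; RaceStall is an interactable stall actor that appears to be the entry point to a race.
; When Player1 overlaps its Box from InGameDay 2 onward, it enables input from the first player controller, and leaving the box disables it.
; Pressing R only sets the FirstTimeRaceEntered flag.
; The node that opens the RaceLvlNew level is unconnected, so the stall itself does not load the race.
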(event OnComponentBeginOverlap(Box)
  (params (OverlappedComponent :type Primitive%20Component%20Object%20Reference) (OtherActor :type Actor%20Object%20Reference) (OtherComp :type Primitive%20Component%20Object%20Reference) (OtherBodyIndex :type Integer) (bFromSweep :type Boolean) (SweepResult :type Hit%20Result%20Structure%20%28by%20ref%29))
  (bind _asplayer_1 (Utilities|Casting|CastToPlayer1 OtherActor))
  (if (not (< (Variables|/Game/Blueprints/Player1.Player1_C|GetinGameDay _asplayer_1) 2))
    (Input|EnableInput (Game|GetPlayerController 0))))

(event OnComponentEndOverlap(Box)
  (params (OverlappedComponent :type Primitive%20Component%20Object%20Reference) (OtherActor :type Actor%20Object%20Reference) (OtherComp :type Primitive%20Component%20Object%20Reference) (OtherBodyIndex :type Integer))
  (Utilities|Casting|CastToPlayer1 OtherActor)
  (Input|DisableInput (Game|GetPlayerController 0)))

(event Input|KeyboardEvents|R
  (params (Key :type Key%20Structure :default "None"))
  (:Pressed
    (Variables|Default|SetfirstTimeRaceEntered true)))

(fn ConstructionScript)