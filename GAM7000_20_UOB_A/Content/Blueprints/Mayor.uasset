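; Mayor NPC that accepts gifts from the player and switches dialogue as the in-game days progress.
; A box overlap toggles input so F can give a held berry or flower, raising Happiness and Mayor social, hiding held items and clearing the held flag.
; Once spoken to, Tick uses a DoOnce and delay to set the dialogue tree for the day cached after BeginPlay, re-checking garden and Day 5 progress flags.
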(event OnComponentBeginOverlap(Box)
  (params (OverlappedComponent :type Primitive%20Component%20Object%20Reference) (OtherActor :type Actor%20Object%20Reference) (OtherComp :type Primitive%20Component%20Object%20Reference) (OtherBodyIndex :type Integer) (bFromSweep :type Boolean) (SweepResult :type Hit%20Result%20Structure%20%28by%20ref%29))
  ;[1 1 1] Enable/Disable Player Input
  (Input|EnableInput (.ReturnValue (Class|VictoryBPFunctionLibrary|AccessorGetPlayerController (Game|GetPlayerCharacter 0)))))

(event OnComponentEndOverlap(Box)
  (params (OverlappedComponent :type Primitive%20Component%20Object%20Reference) (OtherActor :type Actor%20Object%20Reference) (OtherComp :type Primitive%20Component%20Object%20Reference) (OtherBodyIndex :type Integer))
  ;[1 1 1] Enable/Disable Player Input
  (Input|DisableInput (.ReturnValue (Class|VictoryBPFunctionLibrary|AccessorGetPlayerController (Game|GetPlayerCharacter 0)))))

(event EventBeginPlay
  (bind _asplayer_1 (Utilities|Casting|CastToPlayer1 (Game|GetPlayerCharacter 0)))
  (Variables|Default|SetCharacterReference _asplayer_1)
  (Utilities|FlowControl|Delay 1.0)
  (Variables|Default|SetDay (Variables|/Game/Blueprints/Player1.Player1_C|GetinGameDay _asplayer_1)))

(event EventTick
  (params (DeltaSeconds :type Float%20%28single-precision%29))
  (if (Variables|Default|GethasBeenSpokenTo)
    (Utilities|FlowControl|DoOnce false :!label _label
      (:Completed
        (Utilities|FlowControl|Delay 3.0)
        (if (== (Variables|Default|GetDay) 1)
          (Variables|/Game/NewDialogueSystem/NewDialogueComponent.NewDialogueComponent_C|SetDialogueTree (Variables|Default|GetDialogueComponent) "/Game/NewDialogueSystem/DialogueTrees/Day1/Default/MayorDialogueTreeD1_Default.MayorDialogueTreeD1_Default")
          (elif (== (Variables|Default|GetDay) 2)
            (Variables|/Game/NewDialogueSystem/NewDialogueComponent.NewDialogueComponent_C|SetDialogueTree (Variables|Default|GetDialogueComponent) "/Game/NewDialogueSystem/DialogueTrees/Day2/Default/MayorDialogueTreeD2_Default.MayorDialogueTreeD2_Default")
            (elif (== (Variables|Default|GetDay) 3)
              (if (Variables|/Game/Blueprints/Gardening.Gardening_C|GetgardenedFirstTime (Variables|Default|GetGardenRef))
                (Variables|/Game/NewDialogueSystem/NewDialogueComponent.NewDialogueComponent_C|SetDialogueTree (Variables|Default|GetDialogueComponent) "/Game/NewDialogueSystem/DialogueTrees/Day3/Narrative/MayorDialogueTreeD3.MayorDialogueTreeD3")
                (else
                  (Variables|/Game/NewDialogueSystem/NewDialogueComponent.NewDialogueComponent_C|SetDialogueTree (Variables|Default|GetDialogueComponent) "/Game/NewDialogueSystem/DialogueTrees/Day3/Default/MayorDialogueTreeD3_Default.MayorDialogueTreeD3_Default")
                  (goto _label Reset)))
              (elif (== (Variables|Default|GetDay) 4)
                (Variables|/Game/NewDialogueSystem/NewDialogueComponent.NewDialogueComponent_C|SetDialogueTree (Variables|Default|GetDialogueComponent) "/Game/NewDialogueSystem/DialogueTrees/Day4/Default/MayorDialogueTreeD4_Default.MayorDialogueTreeD4_Default")
                (elif (== (Variables|Default|GetDay) 5)
                  (if (Variables|Default|Getday5SecondPortionDialogue)
                    (Variables|/Game/NewDialogueSystem/NewDialogueComponent.NewDialogueComponent_C|SetDialogueTree (Variables|Default|GetDialogueComponent) "/Game/NewDialogueSystem/DialogueTrees/Day5/Narrative/MayorDialogueTreeD5_2.MayorDialogueTreeD5_2")
                    (else
                      (Variables|/Game/NewDialogueSystem/NewDialogueComponent.NewDialogueComponent_C|SetDialogueTree (Variables|Default|GetDialogueComponent) "/Game/NewDialogueSystem/DialogueTrees/Day5/Default/MayorDialogueTreeD5_Default.MayorDialogueTreeD5_Default")
                      (goto _label Reset))))))))))))

(event Input|KeyboardEvents|F
  (params (Key :type Key%20Structure :default "None"))
  (bind _characterreference (Variables|Default|GetCharacterReference))
  (bind _characterreference_2 (Variables|Default|GetCharacterReference))
  (bind _characterreference_3 (Variables|Default|GetCharacterReference))
  ;[1 1 1] Give Held Berry
  (:Pressed
    (Development|PrintString "Pressed F")
    (if (Variables|/Game/Blueprints/Player1.Player1_C|GetHoldingBlackBerry? _characterreference_2)
      (Development|PrintString "Holding Blackberry")
      (Development|PrintString "Given Detective a gift" :!label _label)
      ;[1 1 1] Adding To Happiness/Social Stat
      (bind _asplayer_1 (Utilities|Casting|CastToPlayer1 (Game|GetPlayerCharacter 0))
        (:then
          (Default|Plus1toHappiness _asplayer_1)
          (Default|Plus1toMayorSocial _asplayer_1)
          (Rendering|SetVisibility (Variables|/Game/Blueprints/Player1.Player1_C|GetBlackberry _asplayer_1) false false)
          (if (Variables|/Game/Blueprints/Player1.Player1_C|GetHoldingBlackBerry? _characterreference_3)
            (Variables|/Game/Blueprints/Player1.Player1_C|SetHoldingBlackBerry? _characterreference_3 false)
            (elif (Variables|/Game/Blueprints/Player1.Player1_C|GetHoldingBlueBerry? _characterreference_3)
              (Variables|/Game/Blueprints/Player1.Player1_C|SetHoldingBlueBerry? _characterreference_3 false)
              (elif (Variables|/Game/Blueprints/Player1.Player1_C|GetHoldingRaspBerry? _characterreference_3)
                (Variables|/Game/Blueprints/Player1.Player1_C|SetHoldingRaspBerry? _characterreference_3 false)
                (elif (Variables|/Game/Blueprints/Player1.Player1_C|GetHoldingPoppy? _characterreference_3)
                  (Variables|/Game/Blueprints/Player1.Player1_C|SetHoldingPoppy? _characterreference_3 false)
                  (elif (Variables|/Game/Blueprints/Player1.Player1_C|GetHoldingLotV? _characterreference_3)
                    (Variables|/Game/Blueprints/Player1.Player1_C|SetHoldingLotV? _characterreference_3 false)
                    (elif (Variables|/Game/Blueprints/Player1.Player1_C|GetHoldingFoxglove? _characterreference_3)
                      (Variables|/Game/Blueprints/Player1.Player1_C|SetHoldingFoxglove? _characterreference_3 false))))))))
        (:CastFailed
          (Development|PrintString "Not Working")))
      (elif (Variables|/Game/Blueprints/Player1.Player1_C|GetHoldingBlueBerry? _characterreference_2)
        (Development|PrintString "Holding Blueberry")
        (goto _label)
        (elif (Variables|/Game/Blueprints/Player1.Player1_C|GetHoldingRaspBerry? _characterreference_2)
          (Development|PrintString "Holding Raspberry")
          (goto _label)
          (else
            ;[1 1 1] Give Held Flower
            (if (Variables|/Game/Blueprints/Player1.Player1_C|GetHoldingPoppy? _characterreference)
              (goto _label)
              (elif (Variables|/Game/Blueprints/Player1.Player1_C|GetHoldingLotV? _characterreference)
                (goto _label)
                (elif (Variables|/Game/Blueprints/Player1.Player1_C|GetHoldingFoxglove? _characterreference)
                  (goto _label))))))))))

(fn ConstructionScript)