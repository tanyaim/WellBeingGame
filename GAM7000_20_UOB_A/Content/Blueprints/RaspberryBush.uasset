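; Harvestable raspberry bush that the player picks with F to complete a task and gain happiness.
; A box overlap toggles the bush's input, and a HasBerries flag limits picking to when berries are available.
; Harvesting destroys the four berry spheres, sets Player1's collection flags and hides the journal's URaspberry element on first collection.
; On in-game day 4 it also notifies DoctorRef that the player collected berries.
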(event OnComponentBeginOverlap(Box)
  (params (OverlappedComponent :type Primitive%20Component%20Object%20Reference) (OtherActor :type Actor%20Object%20Reference) (OtherComp :type Primitive%20Component%20Object%20Reference) (OtherBodyIndex :type Integer) (bFromSweep :type Boolean) (SweepResult :type Hit%20Result%20Structure%20%28by%20ref%29))
  ;[1 1 1] Enable/Disable Player Input
  (Input|EnableInput (.ReturnValue (Class|VictoryBPFunctionLibrary|AccessorGetPlayerController (Game|GetPlayerCharacter 0)))))

(event OnComponentEndOverlap(Box)
  (params (OverlappedComponent :type Primitive%20Component%20Object%20Reference) (OtherActor :type Actor%20Object%20Reference) (OtherComp :type Primitive%20Component%20Object%20Reference) (OtherBodyIndex :type Integer))
  ;[1 1 1] Enable/Disable Player Input
  (Input|DisableInput (.ReturnValue (Class|VictoryBPFunctionLibrary|AccessorGetPlayerController (Game|GetPlayerCharacter 0)))))

(event EventBeginPlay
  (bind _asplayer_1 (Utilities|Casting|CastToPlayer1 (Game|GetPlayerCharacter 0)))
  (Variables|Default|SetCharacterReference _asplayer_1))

(event Input|KeyboardEvents|F
  (params (Key :type Key%20Structure :default "None"))
  (bind _characterreference (Variables|Default|GetCharacterReference))
  ;[1 1 1] Completing Task
  (:Pressed
    (if (Variables|Default|GetHasBerries?)
      (Variables|Default|SetHasBerries? false)
      (Variables|Default|SetTaskCompleted? true)
      (Development|PrintString "Task Completed")
      ;[1 1 1] Adding To Happiness
      (bind _asplayer_1 (Utilities|Casting|CastToPlayer1 (Game|GetPlayerCharacter 0))
        (:then
          (Default|Plus1toHappiness _asplayer_1)
          (if (Variables|/Game/Blueprints/Player1.Player1_C|GethasCollectedRaspberry _characterreference)
            _
            (else
              (Class|Image|SetOpacity (Variables|/Game/Journal/Journal.Journal_C|Getu_raspberry (Variables|/Game/Blueprints/Player1.Player1_C|GetJournalReference _characterreference)) 0.0)
              (Variables|/Game/Blueprints/Player1.Player1_C|SethasCollectedRaspberry _characterreference true)))
          (Components|DestroyComponent (Variables|Default|GetSphere))
          (Utilities|FlowControl|Sequence
            (:then_0
              (Utilities|FlowControl|DoOnce false
                (:Completed
                  (Variables|/Game/Blueprints/Player1.Player1_C|SetcollectedRaspberryFirstTime (Variables|Default|GetCharacterReference) true))))
            (:then_1
              (Variables|Default|SetcollectedBerries true)
              (if (== (Variables|/Game/Blueprints/Player1.Player1_C|GetinGameDay (Variables|Default|GetCharacterReference)) 4)
                (Variables|/Game/Blueprints/Doctor.Doctor_C|Setday4BerriesCollectedByPlayer (Variables|Default|GetDoctorRef) true)))))
        (:CastFailed
          (Development|PrintString "Not Working")))
      (else
        (Development|PrintString "Not in harvest")))))

(fn ConstructionScript)