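; GardeningSparkles is a Blueprint holding a set of sparkle particle effects, apparently for gardening, that can be revealed on demand.
; TurnSparklesOn makes all 46 particle system components visible through individual SetVisibility calls, without propagating to children.
; The construction script is empty, and the file shows no function to hide the sparkles or any caller that triggers them.
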(fn ConstructionScript)

(fn TurnSparkleson
  (Rendering|SetVisibility (Variables|Default|GetParticleSystem) true false)
  (Rendering|SetVisibility (Variables|Default|GetParticleSystem1) true false)
  (Rendering|SetVisibility (Variables|Default|GetParticleSystem2) true false)
  (Rendering|SetVisibility (Variables|Default|GetParticleSystem3) true false)
  (Rendering|SetVisibility (Variables|Default|GetParticleSystem4) true false)
  (Rendering|SetVisibility (Variables|Default|GetParticleSystem5) true false)
  (Rendering|SetVisibility (Variables|Default|GetParticleSystem6) true false)
  (Rendering|SetVisibility (Variables|Default|GetParticleSystem7) true false)
  (Rendering|SetVisibility (Variables|Default|GetParticleSystem8) true false)
  (Rendering|SetVisibility (Variables|Default|GetParticleSystem9) true false)
  (Rendering|SetVisibility (Variables|Default|GetParticleSystem10) true false)
  (Rendering|SetVisibility (Variables|Default|GetParticleSystem11) true false)
  (Rendering|SetVisibility (Variables|Default|GetParticleSystem12) true false)
  (Rendering|SetVisibility (Variables|Default|GetParticleSystem13) true false)
  (Rendering|SetVisibility (Variables|Default|GetParticleSystem14) true false)
  (Rendering|SetVisibility (Variables|Default|GetParticleSystem15) true false)
  (Rendering|SetVisibility (Variables|Default|GetParticleSystem16) true false)
  (Rendering|SetVisibility (Variables|Default|GetParticleSystem17) true false)
  (Rendering|SetVisibility (Variables|Default|GetParticleSystem18) true false)
  (Rendering|SetVisibility (Variables|Default|GetParticleSystem19) true false)
  (Rendering|SetVisibility (Variables|Default|GetParticleSystem20) true false)
  (Rendering|SetVisibility (Variables|Default|GetParticleSystem21) true false)
  (Rendering|SetVisibility (Variables|Default|GetParticleSystem22) true false)
  (Rendering|SetVisibility (Variables|Default|GetParticleSystem23) true false)
  (Rendering|SetVisibility (Variables|Default|GetParticleSystem24) true false)
  (Rendering|SetVisibility (Variables|Default|GetParticleSystem25) true false)
  (Rendering|SetVisibility (Variables|Default|GetParticleSystem26) true false)
  (Rendering|SetVisibility (Variables|Default|GetParticleSystem27) true false)
  (Rendering|SetVisibility (Variables|Default|GetParticleSystem28) true false)
  (Rendering|SetVisibility (Variables|Default|GetParticleSystem29) true false)
  (Rendering|SetVisibility (Variables|Default|GetParticleSystem30) true false)
  (Rendering|SetVisibility (Variables|Default|GetParticleSystem31) true false)
  (Rendering|SetVisibility (Variables|Default|GetParticleSystem32) true false)
  (Rendering|SetVisibility (Variables|Default|GetParticleSystem33) true false)
  (Rendering|SetVisibility (Variables|Default|GetParticleSystem34) true false)
  (Rendering|SetVisibility (Variables|Default|GetParticleSystem35) true false)
  (Rendering|SetVisibility (Variables|Default|GetParticleSystem36) true false)
  (Rendering|SetVisibility (Variables|Default|GetParticleSystem37) true false)
  (Rendering|SetVisibility (Variables|Default|GetParticleSystem38) true false)
  (Rendering|SetVisibility (Variables|Default|GetParticleSystem39) true false)
  (Rendering|SetVisibility (Variables|Default|GetParticleSystem40) true false)
  (Rendering|SetVisibility (Variables|Default|GetParticleSystem41) true false)
  (Rendering|SetVisibility (Variables|Default|GetParticleSystem42) true false)
  (Rendering|SetVisibility (Variables|Default|GetParticleSystem43) true false)
  (Rendering|SetVisibility (Variables|Default|GetParticleSystem44) true false)
  (Rendering|SetVisibility (Variables|Default|GetParticleSystem45) true false))