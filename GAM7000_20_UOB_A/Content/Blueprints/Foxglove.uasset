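; Foxglove is a collectible pickup that records its collection on the Player1 character.
; Its Box overlap events enable and disable the actor's input for the first player controller, without checking which actor overlaps.
; Releasing F sets PickedUpFoxglove on the cached player reference.
; A DoOnce then sets CollectedFoxgloveFirstTime and destroys the Box and Cube components, leaving the actor itself in place.
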(event OnComponentBeginOverlap(Box)
  (params (OverlappedComponent :type Primitive%20Component%20Object%20Reference) (OtherActor :type Actor%20Object%20Reference) (OtherComp :type Primitive%20Component%20Object%20Reference) (OtherBodyIndex :type Integer) (bFromSweep :type Boolean) (SweepResult :type Hit%20Result%20Structure%20%28by%20ref%29))
  ;[1 1 1] Enable/Disable Player Input
  (Input|EnableInput (.ReturnValue (Class|VictoryBPFunctionLibrary|AccessorGetPlayerController (Game|GetPlayerCharacter 0)))))

(event OnComponentEndOverlap(Box)
  (params (OverlappedComponent :type Primitive%20Component%20Object%20Reference) (OtherActor :type Actor%20Object%20Reference) (OtherComp :type Primitive%20Component%20Object%20Reference) (OtherBodyIndex :type Integer))
  ;[1 1 1] Enable/Disable Player Input
  (Input|DisableInput (.ReturnValue (Class|VictoryBPFunctionLibrary|AccessorGetPlayerController (Game|GetPlayerCharacter 0)))))

(event EventBeginPlay
  (bind _asplayer_1 (Utilities|Casting|CastToPlayer1 (Game|GetPlayerCharacter 0)))
  (Variables|Default|SetPlayerRef _asplayer_1))

(event Input|KeyboardEvents|F
  (params (Key :type Key%20Structure :default "None"))
  (bind _playerref (Variables|Default|GetPlayerRef))
  ;[1 1 1] Pick Up Poppy
  (:Released
    (Variables|/Game/Blueprints/Player1.Player1_C|SetPickedUpFoxglove? _playerref true)
    (Utilities|FlowControl|DoOnce false
      (:Completed
        (Variables|/Game/Blueprints/Player1.Player1_C|SetcollectedFoxgloveFirstTime _playerref true)
        (Components|DestroyComponent (Variables|Default|GetBox))))))

(fn ConstructionScript)