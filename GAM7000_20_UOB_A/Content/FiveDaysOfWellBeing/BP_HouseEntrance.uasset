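; BP_HouseEntrance is an interactable entrance that saves the player's progress and opens the level matching the current in-game day.
; Its box overlap enables input only while Player1 is inside.
; BeginPlay caches the player and creates a fresh Variables_Save object.
; Pressing E copies collection flags, social values and the day into that save, writes the PlayerVariables slot, then branches on the day, ending at AfterNarrative on day five.
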(event OnComponentBeginOverlap(Box)
  (params (OverlappedComponent :type Primitive%20Component%20Object%20Reference) (OtherActor :type Actor%20Object%20Reference) (OtherComp :type Primitive%20Component%20Object%20Reference) (OtherBodyIndex :type Integer) (bFromSweep :type Boolean) (SweepResult :type Hit%20Result%20Structure%20%28by%20ref%29))
  (Utilities|Casting|CastToPlayer1 OtherActor)
  (Input|EnableInput (Game|GetPlayerController 0)))

(event OnComponentEndOverlap(Box)
  (params (OverlappedComponent :type Primitive%20Component%20Object%20Reference) (OtherActor :type Actor%20Object%20Reference) (OtherComp :type Primitive%20Component%20Object%20Reference) (OtherBodyIndex :type Integer))
  (Utilities|Casting|CastToPlayer1 OtherActor)
  (Input|DisableInput (Game|GetPlayerController 0)))

(event EventBeginPlay
  (bind _asplayer_1 (Utilities|Casting|CastToPlayer1 (Game|GetPlayerCharacter 0)))
  (Variables|Default|SetPlayerReference _asplayer_1)
  (bind _returnvalue (SaveGame|CreateSaveGameObject "/Game/SavingValues/Variables_Save.Variables_Save_C"))
  (Variables|Default|SetSaveGameReference _returnvalue)
  (Utilities|FlowControl|Delay 1.0)
  (Variables|Default|SetDay (Variables|/Game/Blueprints/Player1.Player1_C|GetinGameDay (Variables|Default|GetPlayerReference))))

(event Input|KeyboardEvents|E
  (params (Key :type Key%20Structure :default "None"))
  (bind _playerreference (Variables|Default|GetPlayerReference))
  (bind _savegamereference (Variables|Default|GetSaveGameReference))
  (:Pressed
    (SaveGame|SaveGametoSlot (Variables|Default|GetSaveGameReference) "PlayerVariables")
    (Variables|/Game/SavingValues/Variables_Save.Variables_Save_C|SethasBlackberry _savegamereference (Variables|/Game/Blueprints/Player1.Player1_C|GetcollectedBlackberryFirstTime _playerreference))
    (Variables|/Game/SavingValues/Variables_Save.Variables_Save_C|SethasBlueberry _savegamereference (Variables|/Game/Blueprints/Player1.Player1_C|GetcollectedBlueberryFristTime _playerreference))
    (Variables|/Game/SavingValues/Variables_Save.Variables_Save_C|SethasRaspberry _savegamereference (Variables|/Game/Blueprints/Player1.Player1_C|GetcollectedRaspberryFirstTime _playerreference))
    (Variables|/Game/SavingValues/Variables_Save.Variables_Save_C|SethasPoppy _savegamereference (Variables|/Game/Blueprints/Player1.Player1_C|GetcollectedPoppyFirstTime _playerreference))
    (Variables|/Game/SavingValues/Variables_Save.Variables_Save_C|SethasLotV _savegamereference (Variables|/Game/Blueprints/Player1.Player1_C|GetcollectedLotVFirstTime _playerreference))
    (Variables|/Game/SavingValues/Variables_Save.Variables_Save_C|SethasFoxglove _savegamereference (Variables|/Game/Blueprints/Player1.Player1_C|GetcollectedFoxgloveFirstTime _playerreference))
    (Variables|/Game/SavingValues/Variables_Save.Variables_Save_C|SetMayorSocial _savegamereference (Variables|/Game/Blueprints/Player1.Player1_C|GetMayorSocial _playerreference))
    (Variables|/Game/SavingValues/Variables_Save.Variables_Save_C|SetDetectiveSocial _savegamereference (Variables|/Game/Blueprints/Player1.Player1_C|GetDetectiveSocial _playerreference))
    (Variables|/Game/SavingValues/Variables_Save.Variables_Save_C|SetDoctorSocial _savegamereference (Variables|/Game/Blueprints/Player1.Player1_C|GetDoctorSocial _playerreference))
    (Variables|/Game/SavingValues/Variables_Save.Variables_Save_C|SetChefSocial _savegamereference (Variables|/Game/Blueprints/Player1.Player1_C|GetChefSocial _playerreference))
    (bind _output_get (Variables|/Game/SavingValues/Variables_Save.Variables_Save_C|SetinGameDay _savegamereference (Variables|/Game/Blueprints/Player1.Player1_C|GetinGameDay _playerreference)))
    (SaveGame|SaveGametoSlot (Variables|Default|GetSaveGameReference) "PlayerVariables")
    (if (== _output_get 1)
      (Game|OpenLevel(byName) (Variables|Default|Get2))
      (elif (== _output_get 2)
        (Game|OpenLevel(byName) (Variables|Default|Get3))
        (elif (== _output_get 3)
          (Game|OpenLevel(byName) (Variables|Default|Get4))
          (elif (== _output_get 4)
            (Game|OpenLevel(byName) (Variables|Default|Get5))
            (elif (== _output_get 5)
              (Game|OpenLevel(byName) (Variables|Default|GetAfterNarrative)))))))))

(fn ConstructionScript)