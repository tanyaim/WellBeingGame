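; BP_ObjDay2BeActive is a quest objective, named for being active on Day 2, that reports whether the player has engaged with its target actor.
; GetIsComplete tries casting ActorToInteractWith to Doctor, Mayor and RaceStall in a Sequence, so the matching type decides the result.
; Doctor and Mayor report whether they have been spoken to, while RaceStall reports its FirstTimeRaceEntered flag.
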(fn GetIsComplete
  (Utilities|FlowControl|Sequence
    (:then_0
      (bind _asdoctor (Utilities|Casting|CastToDoctor (Variables|Default|GetActorToInteractWith)))
      (return (Variables|/Game/Blueprints/Doctor.Doctor_C|GethasBeenSpokenTo _asdoctor)))
    (:then_1
      (bind _asmayor (Utilities|Casting|CastToMayor (Variables|Default|GetActorToInteractWith)))
      (return (Variables|/Game/Blueprints/Mayor.Mayor_C|GethasBeenSpokenTo _asmayor)))
    (:then_2
      (bind _asrace_stall (Utilities|Casting|CastToRaceStall (Variables|Default|GetActorToInteractWith)))
      (return (Variables|/Game/Blueprints/RaceStall.RaceStall_C|GetfirstTimeRaceEntered _asrace_stall)))))