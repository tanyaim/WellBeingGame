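; BP_ObjDay5Give is a quest objective, named for a Day 5 give task, that reports whether its target actor has been dealt with.
; GetIsComplete uses a Sequence of casts on ActorToInteractWith, so the first matching type supplies the result.
; Doctor, Mayor and Chef targets return HasBeenSpokenTo, while a ShopStall target returns GiftPurchased.
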(fn GetIsComplete
  (Utilities|FlowControl|Sequence
    (:then_0
      (bind _asdoctor (Utilities|Casting|CastToDoctor (Variables|Default|GetActorToInteractWith)))
      (return (Variables|/Game/Blueprints/Doctor.Doctor_C|GethasBeenSpokenTo _asdoctor)))
    (:then_1
      (bind _asmayor (Utilities|Casting|CastToMayor (Variables|Default|GetActorToInteractWith)))
      (return (Variables|/Game/Blueprints/Mayor.Mayor_C|GethasBeenSpokenTo _asmayor)))
    (:then_2
      (bind _aschef (Utilities|Casting|CastToChef (Variables|Default|GetActorToInteractWith)))
      (return (Variables|/Game/Blueprints/Chef.Chef_C|GethasBeenSpokenTo _aschef)))
    (:then_3
      (bind _asshop_stall (Utilities|Casting|CastToShopStall (Variables|Default|GetActorToInteractWith)))
      (return (Variables|/Game/QuestSystem/ShopStall.ShopStall_C|GetGiftPurchased _asshop_stall)))))