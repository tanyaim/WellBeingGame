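; BP_ObjDay3TakeNotice is a quest objective, named for a Day 3 "take notice" task, that reports whether the player has completed an interaction with its target actor.
; GetIsComplete tries casting ActorToInteractWith to Detective, Gardening and Mayor in sequence, falling through when a cast fails.
; It returns HasBeenSpokenTo for the Detective or Mayor, and GardenedFirstTime for Gardening.
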(fn GetIsComplete
  (Utilities|FlowControl|Sequence
    (:then_0
      (bind _asdetective (Utilities|Casting|CastToDetective (Variables|Default|GetActorToInteractWith)))
      (return (Variables|/Game/Blueprints/Detective.Detective_C|GethasBeenSpokenTo _asdetective)))
    (:then_1
      (bind _asgardening (Utilities|Casting|CastToGardening (Variables|Default|GetActorToInteractWith)))
      (return (Variables|/Game/Blueprints/Gardening.Gardening_C|GetgardenedFirstTime _asgardening)))
    (:then_2
      (bind _asmayor (Utilities|Casting|CastToMayor (Variables|Default|GetActorToInteractWith)))
      (return (Variables|/Game/Blueprints/Mayor.Mayor_C|GethasBeenSpokenTo _asmayor)))))