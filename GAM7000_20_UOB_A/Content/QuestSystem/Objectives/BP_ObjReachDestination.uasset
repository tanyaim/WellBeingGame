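; BP_ObjReachDestination is a quest objective that completes when the player reaches a Destination actor.
; On activation it runs the parent logic and binds to the Destination's begin-overlap event.
; When a Player1 actor overlaps, it unbinds the event, sets ReachedDestination and calls OnCompleted with itself.
; GetIsComplete reports the ReachedDestination flag.
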(event Custom|OnActorBeginOverlapEvent
  (params (OverlappedActor :type Actor%20Object%20Reference) (OtherActor :type Actor%20Object%20Reference))
  (Utilities|Casting|CastToPlayer1 OtherActor)
  (Collision|UnbindEventfromOnActorBeginOverlap (Variables|Default|GetDestination) (delegate Custom|OnActorBeginOverlapEvent))
  (Variables|Default|SetReachedDestination true)
  (Default|CallOnCompleted self))

(event EventActivateObjective
  (|CallParentFunction)
  (EventDispatchers|AssignOnActorBeginOverlap (Variables|Default|GetDestination) (delegate Custom|OnActorBeginOverlapEvent)))

(fn GetIsComplete
  (return (Variables|Default|GetReachedDestination)))