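; BP_ObjDay1Connect is a quest objective, named for a Day 1 connect task, that completes when its target character has been spoken to.
; GetIsComplete tries casting ActorToInteractWith to Mayor, Detective, Doctor and Chef in sequence, returning the matching character's HasBeenSpokenTo flag.
; ActivateObjective is an empty event, so the completion check is the only logic in the graphs.
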(event EventActivateObjective)

(fn GetIsComplete
  (Utilities|FlowControl|Sequence
    (:then_0
      (bind _asmayor (Utilities|Casting|CastToMayor (Variables|Default|GetActorToInteractWith)))
      (return (Variables|/Game/Blueprints/Mayor.Mayor_C|GethasBeenSpokenTo _asmayor)))
    (:then_1
      (bind _asdetective (Utilities|Casting|CastToDetective (Variables|Default|GetActorToInteractWith)))
      (return (Variables|/Game/Blueprints/Detective.Detective_C|GethasBeenSpokenTo _asdetective)))
    (:then_2
      (bind _asdoctor (Utilities|Casting|CastToDoctor (Variables|Default|GetActorToInteractWith)))
      (return (Variables|/Game/Blueprints/Doctor.Doctor_C|GethasBeenSpokenTo _asdoctor)))
    (:then_3
      (bind _aschef (Utilities|Casting|CastToChef (Variables|Default|GetActorToInteractWith)))
      (return (Variables|/Game/Blueprints/Chef.Chef_C|GethasBeenSpokenTo _aschef)))))