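; Quest objective Blueprint for a Day 4 "Keep Learning" task that decides completion through GetIsComplete.
; A sequence first casts the Doctor reference and returns whether the Doctor has been spoken to.
; A second branch nests loops over blueberry, blackberry and raspberry bushes, returning whether berries were collected from all three current bushes.
; Early returns mean a valid Doctor skips the berry check, and the loops only evaluate each array's first bush.
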(fn GetIsComplete
  (Utilities|FlowControl|Sequence
    (:then_0
      (bind _asdoctor (Utilities|Casting|CastToDoctor (Variables|Default|GetDoctor)))
      (return (Variables|/Game/Blueprints/Doctor.Doctor_C|GethasBeenSpokenTo _asdoctor)))
    (:then_1
      (for _array_element (Variables|Default|GetBlueberryBushes)
        (for _array_element_2 (Variables|Default|GetBlackberryBushes)
          (for _array_element_3 (Variables|Default|GetRaspberryBushes)
            (return (Math|Boolean|ANDBoolean (Variables|/Game/Blueprints/RaspberryBush.RaspberryBush_C|GetcollectedBerries _array_element_3) (Variables|/Game/Blueprints/BlackberryBush.BlackberryBush_C|GetcollectedBerries _array_element_2) (Variables|/Game/Blueprints/BlueberryBush.BlueberryBush_C|GetcollectedBerries _array_element)))))))))