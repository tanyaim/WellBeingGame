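; BP_Quest2 is a quest in the quest system that has the player collect blackberries under an ordered root objective named "Take Notice".
; It overrides ConstructRootObjectiveCollection to create that root BP_ObjCollection with order required.
; PopulateObjectives then adds one BP_ObjCollectBlackBerry per entry in the BlackberryBushes array, each bound to its bush.
; The event graph holds no active logic.
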(event EventBeginPlay
  (|CallParentFunction) ; This node is disabled and will not be called.\nDrag off pins to build functionality.
)

(event Collision|EventActorBeginOverlap
  (params (OtherActor :type Actor%20Object%20Reference)))

(event EventTick
  (params (DeltaSeconds :type Float%20%28single-precision%29)))

(fn ConstructionScript
  (|CallParentFunction))

(fn ConstructRootObjectiveCollection
  (bind _returnvalue (Game|ConstructObjectfromClass "/Game/QuestSystem/Objectives/BP_ObjCollection.BP_ObjCollection_C" self true "Take Notice"))
  (return _returnvalue))

(fn PopulateObjectives
  (params (RootObjCollection :type BP%20Obj%20Collection%20Object%20Reference))
  (for _array_element (Variables|Default|GetBlackberryBushes)
    (bind _returnvalue (Game|ConstructObjectfromClass "/Game/QuestSystem/Objectives/BP_ObjCollectBlackBerry.BP_ObjCollectBlackBerry_C" self _array_element "Collect Blackberries"))
    (Default|AddObjective RootObjCollection _returnvalue)))