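; BP_QuestDay1Connect is the Day 1 "Connect" quest, which has the player meet key townsfolk.
; It builds an order-required BP_ObjCollection as the root objective.
; PopulateObjectives adds one BP_ObjDay1Connect objective each for the Mayor, Detective, Doctor and Chef, in that sequence.
; Each objective reuses the same class, differing only in its target actor and display name.
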(fn ConstructionScript
  (|CallParentFunction))

(fn ConstructRootObjectiveCollection
  (bind _returnvalue (Game|ConstructObjectfromClass "/Game/QuestSystem/Objectives/BP_ObjCollection.BP_ObjCollection_C" self true "Connect:"))
  (return _returnvalue))

(fn PopulateObjectives
  (params (RootObjCollection :type BP%20Obj%20Collection%20Object%20Reference))
  (Utilities|FlowControl|Sequence
    (:then_0
      (bind _returnvalue (Game|ConstructObjectfromClass "/Game/QuestSystem/Objectives/BP_ObjDay1Connect.BP_ObjDay1Connect_C" self (Variables|Default|GetMayor) "Talk to the Mayor"))
      (Default|AddObjective RootObjCollection _returnvalue))
    (:then_1
      (bind _returnvalue_2 (Game|ConstructObjectfromClass "/Game/QuestSystem/Objectives/BP_ObjDay1Connect.BP_ObjDay1Connect_C" self (Variables|Default|GetDetective) "Meet the Detective"))
      (Default|AddObjective RootObjCollection _returnvalue_2))
    (:then_2
      (bind _returnvalue_3 (Game|ConstructObjectfromClass "/Game/QuestSystem/Objectives/BP_ObjDay1Connect.BP_ObjDay1Connect_C" self (Variables|Default|GetDoctor) "Meet the Doctor"))
      (Default|AddObjective RootObjCollection _returnvalue_3))
    (:then_3
      (bind _returnvalue_4 (Game|ConstructObjectfromClass "/Game/QuestSystem/Objectives/BP_ObjDay1Connect.BP_ObjDay1Connect_C" self (Variables|Default|GetChef) "Meet the Chef"))
      (Default|AddObjective RootObjCollection _returnvalue_4))))