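; Day 3 "Take Notice" quest that sends the player to Detective Peacoat, the garden and Mayor Eggbert, in that order.
; It builds a root objective collection with order required, then fills it with three objectives of one shared class.
; Each objective differs only in its display name and the actor to interact with.
; The event graph is unused, so the Blueprint only defines the quest's structure.
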(event EventBeginPlay
  (|CallParentFunction) ; This node is disabled and will not be called.\nDrag off pins to build functionality.
)

(event Collision|EventActorBeginOverlap
  (params (OtherActor :type Actor%20Object%20Reference)))

(event EventTick
  (params (DeltaSeconds :type Float%20%28single-precision%29)))

(fn ConstructionScript
  (|CallParentFunction))

(fn ConstructRootObjectiveCollection
  (bind _returnvalue (Game|ConstructObjectfromClass "/Game/QuestSystem/Objectives/BP_ObjCollection.BP_ObjCollection_C" self true "Take Notice:"))
  (return _returnvalue))

(fn PopulateObjectives
  (params (RootObjCollection :type BP%20Obj%20Collection%20Object%20Reference))
  (Utilities|FlowControl|Sequence
    (:then_0
      (bind _returnvalue (Game|ConstructObjectfromClass "/Game/QuestSystem/Objectives/BP_ObjDay3TakeNotice.BP_ObjDay3TakeNotice_C" self (Variables|Default|GetDetective) "1. Speak to Detective Peacoat"))
      (Default|AddObjective RootObjCollection _returnvalue))
    (:then_1
      (bind _returnvalue_2 (Game|ConstructObjectfromClass "/Game/QuestSystem/Objectives/BP_ObjDay3TakeNotice.BP_ObjDay3TakeNotice_C" self (Variables|Default|GetGardeningGame) "2. Visit the garden"))
      (Default|AddObjective RootObjCollection _returnvalue_2))
    (:then_2
      (bind _returnvalue_3 (Game|ConstructObjectfromClass "/Game/QuestSystem/Objectives/BP_ObjDay3TakeNotice.BP_ObjDay3TakeNotice_C" self (Variables|Default|GetMayor) "3. Speak To Mayor Eggbert"))
      (Default|AddObjective RootObjCollection _returnvalue_3))))