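; Day 2 "Be Active" quest that has the player speak to Doctor Humbug, speak to the Mayor, then enter a race.
; It builds an order-required objective collection as the root, then fills it with three instances of the same objective class, BP_ObjDay2BeActive.
; Each instance differs only in its display name and the actor to interact with: Doctor, Mayor or RaceStall.
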(fn ConstructionScript
  (|CallParentFunction))

(fn ConstructRootObjectiveCollection
  (bind _returnvalue (Game|ConstructObjectfromClass "/Game/QuestSystem/Objectives/BP_ObjCollection.BP_ObjCollection_C" self true "Be Active:"))
  (return _returnvalue))

(fn PopulateObjectives
  (params (RootObjCollection :type BP%20Obj%20Collection%20Object%20Reference))
  (Utilities|FlowControl|Sequence
    (:then_0
      (bind _returnvalue (Game|ConstructObjectfromClass "/Game/QuestSystem/Objectives/BP_ObjDay2BeActive.BP_ObjDay2BeActive_C" self (Variables|Default|GetDoctor) "1. Speak To Doctor Humbug"))
      (Default|AddObjective RootObjCollection _returnvalue))
    (:then_1
      (bind _returnvalue_2 (Game|ConstructObjectfromClass "/Game/QuestSystem/Objectives/BP_ObjDay2BeActive.BP_ObjDay2BeActive_C" self (Variables|Default|GetMayor) "2. Speak To Mayor"))
      (Default|AddObjective RootObjCollection _returnvalue_2))
    (:then_2
      (bind _returnvalue_3 (Game|ConstructObjectfromClass "/Game/QuestSystem/Objectives/BP_ObjDay2BeActive.BP_ObjDay2BeActive_C" self (Variables|Default|GetRaceStall) "3. Enter race"))
      (Default|AddObjective RootObjCollection _returnvalue_3))))