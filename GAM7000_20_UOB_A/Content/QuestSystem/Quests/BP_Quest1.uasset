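; BP_Quest1 is a quest definition whose goal is to reach town.
; It overrides objective construction to create an ordered BP_ObjCollection root labelled "Connect:".
; It then populates that root with a single BP_ObjReachDestination objective that targets the TownTrigger reference.
; Its event graph holds only disabled default nodes, so all of its own logic lives in those two functions.
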(event EventBeginPlay
  (|CallParentFunction) ; This node is disabled and will not be called.\nDrag off pins to build functionality.
)

(event Collision|EventActorBeginOverlap
  (params (OtherActor :type Actor%20Object%20Reference)))

(event EventTick
  (params (DeltaSeconds :type Float%20%28single-precision%29)))

(fn ConstructionScript
  (|CallParentFunction))

(fn ConstructRootObjectiveCollection
  (bind _returnvalue (Game|ConstructObjectfromClass "/Game/QuestSystem/Objectives/BP_ObjCollection.BP_ObjCollection_C" self true "Connect:"))
  (return _returnvalue))

(fn PopulateObjectives
  (params (RootObjCollection :type BP%20Obj%20Collection%20Object%20Reference))
  (bind _returnvalue (Game|ConstructObjectfromClass "/Game/QuestSystem/Objectives/BP_ObjReachDestination.BP_ObjReachDestination_C" self (Variables|Default|GetTownTrigger) "Reach Town"))
  (Default|AddObjective RootObjCollection _returnvalue))